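; Showcase actor that loops a swordsman's sweep animation to demo impact particle effects.
; After an initial delay, a looping timer replays the animation on the skeletal mesh.
; Each sweep runs three separately delayed hits, each spawning its own emitter template at the sword's TipTop socket, oriented by the actor's rotation plus a fixed offset.
; Each hit deactivates its previous emitter before spawning the next.
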(event `self.ReceiveBeginPlay`
  ;[1 1 1] Original by Salty Panda, butchered by Luos
  (`KismetSystemLibrary.Delay` (`self.InitialDelay`))
  ;[1 1 1] LuosArts -- Start Anim - Sword Sweep
  (`self.SwordSweep`)
  (`KismetSystemLibrary.K2_SetTimerDelegate` (delegate `SwordSweep`) (`self.LoopTime`) true))

(event `SwordSweep`
  (bind _spawnedfx_3 (`self.SpawnedFX_3`))
  (bind _spawnedfx_1 (`self.SpawnedFX_1`))
  (bind _spawnedfx_2 (`self.SpawnedFX_2`))
  ;[1 1 1] LuosArts -- Start Anim - Sword Sweep
  (`SkeletalMeshComponent.PlayAnimation` (`self.SK_Swordguy_01`) "/Game/ImpactFX/Z_Showcase/AnimGuy/SkeletalMeshes/SK_Swordguy_01_Anim.SK_Swordguy_01_Anim" false)
  ;[1 1 1] FX Sequence
  (`|ExecutionSequence`
    (:`then_0`
      (`KismetSystemLibrary.Delay` (`self.HitDelay_1`))
      (`/Engine/EditorBlueprintResources/StandardMacros.IsValid` _spawnedfx_1
        (:`Is Valid`
          (`ActorComponent.Deactivate` _spawnedfx_1))
        (:`Is Not Valid`
          _))
      (bind _returnvalue (`GameplayStatics.SpawnEmitterAtLocation` (`self.Template`) (`SceneComponent.GetSocketLocation` (`self.SM_SwordSweepSword_01`) "TipTop") (`KismetMathLibrary.ComposeRotators` (`self.K2_GetActorRotation`) (struct :`Yaw` 90.0))))
      (set `self.SpawnedFX_1` _returnvalue))
    (:`then_1`
      (`KismetSystemLibrary.Delay` (`self.HitDelay_2`))
      (`/Engine/EditorBlueprintResources/StandardMacros.IsValid` _spawnedfx_2
        (:`Is Valid`
          (`ActorComponent.Deactivate` _spawnedfx_2))
        (:`Is Not Valid`
          _))
      (bind _returnvalue_2 (`GameplayStatics.SpawnEmitterAtLocation` (`self.Template_b`) (`SceneComponent.GetSocketLocation` (`self.SM_SwordSweepSword_01`) "TipTop") (`KismetMathLibrary.ComposeRotators` (`self.K2_GetActorRotation`) (struct :`Yaw` 90.0))))
      (set `self.SpawnedFX_2` _returnvalue_2))
    (:`then_2`
      (`KismetSystemLibrary.Delay` (`self.HitDelay_3`))
      (`/Engine/EditorBlueprintResources/StandardMacros.IsValid` _spawnedfx_3
        (:`Is Valid`
          (`ActorComponent.Deactivate` _spawnedfx_3))
        (:`Is Not Valid`
          _))
      (bind _returnvalue_3 (`GameplayStatics.SpawnEmitterAtLocation` (`self.Template_c`) (`SceneComponent.GetSocketLocation` (`self.SM_SwordSweepSword_01`) "TipTop") (`KismetMathLibrary.ComposeRotators` (`self.K2_GetActorRotation`) (struct :`Yaw` 90.0))))
      (set `self.SpawnedFX_3` _returnvalue_3))))

(fn `UserConstructionScript`)