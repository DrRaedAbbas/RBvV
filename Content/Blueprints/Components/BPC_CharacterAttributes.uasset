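; Character attribute component that tracks Health and Rage and exposes getters for both.
; Rage regenerates on a Tick, whose interval comes from the Stamina variable, and stays clamped between empty and full.
; TakeDamage subtracts Health and sends the owner a death message with the killer at zero, unless a takedown is active.
; DeductRage works only during a takedown, throttled by a DoOnce that resets after a short delay.
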(event `self.ReceiveBeginPlay`
  (`self.SetComponentTickInterval` (`self.Stamina`)))

(event `self.ReceiveTick`
  (params (DeltaSeconds :type "Float (single-precision)"))
  (if (< (`self.Rage`) 100.0)
    (`self.AddRage` (`self.RegenarationRageValue`))))

(event `SetIsTakedown`
  (params (`IsTakedown?` :type Boolean))
  (set `self.IsTakedown?` `IsTakedown?`))

(event `TakeDamage`
  (params (`Damage Taken` :type "Float (double-precision)") (Killer :type "Actor Object Reference"))
  (bind _output_get (set `self.Health` (- (`self.Health`) `Damage Taken`)))
  (if (<= _output_get 0.0)
    (if (not (`self.IsTakedown?`))
      (message `/Game/Blueprints/Interfaces/BPI_CharacterAttributes.Set Is Dead` (`self.GetOwner`) true Killer))))

(event `AddRage`
  (params (RageValue :type "Float (double-precision)"))
  (set `self.Rage` (`KismetMathLibrary.FClamp` (+ (`self.Rage`) RageValue) 0.0 100.0)))

(event `DeductRage`
  (params (RageValue :type "Float (double-precision)"))
  (if (`self.IsTakedown?`)
    (`/Engine/EditorBlueprintResources/StandardMacros.DoOnce` false :!label _label
      (:`Completed`
        (set `self.Rage` (`KismetMathLibrary.FClamp` (- (`self.Rage`) RageValue) 0.0 100.0))
        (`KismetSystemLibrary.Delay` 1.0)
        (goto _label :!via `Reset`)))))

(fn `ReturnCurrentHealth`
  (returns (CurrentHealth :type "Float (double-precision)"))
  (return (`self.Health`)))

(fn `ReturnCurrentRage`
  (returns (CurrentRage :type "Float (double-precision)"))
  (return (`self.Rage`)))