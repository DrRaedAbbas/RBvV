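; BP_Camera is a shared camera that follows all player-controlled characters and zooms to their spread.
; After a BeginPlay delay, it becomes every BP_RBvV_PC's view target and collects player characters from the game mode.
; Each tick, authority targets their average location, or the lone character's, and derives a clamped spring arm length from their largest pairwise distance.
; Authority and remote instances both lerp position and arm length toward those targets.
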(event `self.ReceiveBeginPlay`
  (`KismetSystemLibrary.Delay` 2.0)
  (bind _asbp_rbv_v_gm (cast `/Game/Blueprints/BP_RBvV_GM` (`GameplayStatics.GetGameMode`))
    (:`then`
      (set `self.RBVV GM` _asbp_rbv_v_gm))
    (:`CastFailed`
      _))
  (`self.UpdatePlayersAndCharacters`))

(event `self.ReceiveTick`
  (params (DeltaSeconds :type "Float (single-precision)"))
  (bind _playercharacters (`self.PlayerCharacters`))
  (bind _springarm (`self.SpringArm`))
  (bind _output (`|GetArrayItem` _playercharacters))
  (`/Engine/EditorBlueprintResources/ActorMacros.Switch Has Authority`
    (:`Authority`
      (set `self.CurrentLocation` (`self.K2_GetActorLocation`))
      (if (> (`KismetArrayLibrary.Array_Length` _playercharacters) 1)
        (bind _returnvalue (`GameplayStatics.GetActorArrayAverageLocation` _playercharacters))
        (set `self.NewLocation` _returnvalue)
        (`self.SetCameraLocation` :!label _label)
        (`self.AdjustSpringArm`)
        (else
          (`/Engine/EditorBlueprintResources/StandardMacros.IsValid` _output
            (:`Is Valid`
              (set `self.NewLocation` (`self.K2_GetActorLocation` _output))
              (goto _label))
            (:`Is Not Valid`
              (set `self.NewLocation` (`self.K2_GetActorLocation`))
              (set `SpringArmComponent.TargetArmLength` (`SpringArmComponent.TargetArmLength` _springarm) _springarm))))))
    (:`Remote`
      (goto _label))))

(fn `AdjustSpringArm`
  (locals (Character :type "Pawn Object Reference") (AllDistances :type "Array of Float (double-precision)"))
  (bind _springarm (`self.SpringArm`))
  (bind _springarm_2 (`self.SpringArm`))
  (`/Engine/EditorBlueprintResources/ActorMacros.Switch Has Authority`
    (:`Authority`
      (for (_array_element _array_index) (`self.PlayerCharacters`)
        (bind _output_get (set `local.Character` _array_element))
        (`/Engine/EditorBlueprintResources/StandardMacros.IsValid` _output_get
          (:`Is Valid`
            (for _index (range (+ (`KismetArrayLibrary.Array_LastIndex` (`self.PlayerCharacters`)) 1))
              (`KismetArrayLibrary.Array_AddUnique` (`local.AllDistances`) (`self.GetDistanceTo` (`local.Character`) (`|GetArrayItem` (`self.PlayerCharacters`) _index)))))))
      (set `self.New Target Arm Length` (`KismetMathLibrary.FClamp` (`.MaxValue` (`KismetMathLibrary.MaxOfFloatArray` (`local.AllDistances`))) (`self.Min Arm Length`) (`self.Max Arm Length`)))
      (set `SpringArmComponent.TargetArmLength` (`KismetMathLibrary.Lerp` (`SpringArmComponent.TargetArmLength` _springarm) (`self.New Target Arm Length`) 0.1) _springarm))
    (:`Remote`
      (set `SpringArmComponent.TargetArmLength` (`KismetMathLibrary.Lerp` (`SpringArmComponent.TargetArmLength` _springarm_2) (`self.New Target Arm Length`) 0.1) _springarm_2))))

(fn `SetCameraLocation`
  (`self.K2_SetActorLocation` (`KismetMathLibrary.VLerp` (`self.CurrentLocation`) (`self.NewLocation`) 0.1)))

(fn `UpdatePlayersAndCharacters`
  (bind _playercharacters (`self.PlayerCharacters`))
  (if (`KismetSystemLibrary.IsDedicatedServer`)
    (`/Engine/EditorBlueprintResources/ActorMacros.Switch Has Authority`
      (:`Authority`
        _)))
  (bind _outactors (`GameplayStatics.GetAllActorsOfClass` "/Game/Blueprints/Characters/BP_RBvV_PC.BP_RBvV_PC_C"))
  (bind _output_get (set `self.PlayerControllers` _outactors))
  (for _array_element _output_get
    (set `/Game/Blueprints/Characters/BP_RBvV_PC.ViewCamera` self _array_element)
    (`PlayerController.SetViewTargetWithBlend` _array_element self 1.0 "VTBlend_Linear" 0.0 true))
  (`KismetArrayLibrary.Array_Clear` (`self.PlayerCharacters`))
  (bind _rbvv_gm (`self.RBVV GM`)
    (:`then`
      (for _array_element_2 (`/Game/Blueprints/BP_RBvV_GM.RBVVCharacters` _rbvv_gm)
        (if (`Pawn.IsPlayerControlled` _array_element_2)
          (cast `/Game/Blueprints/Characters/BP_RBvV_PC` (`Pawn.GetController` _array_element_2))
          (`KismetArrayLibrary.Array_AddUnique` _playercharacters _array_element_2)
          (else
            (`KismetArrayLibrary.Array_RemoveItem` _playercharacters _array_element_2))))
      (return))
    (:`else`)))

(fn `UserConstructionScript`)