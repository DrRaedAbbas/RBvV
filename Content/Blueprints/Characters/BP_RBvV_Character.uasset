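; Base RBvV character that a player or AI can control, tracking availability and updating its HUD player name on possession.
; Punch, kick and random takedown attacks go through SRV events into an ability component, while inputs move and jump only when movement is allowed.
; Hit reactions and death route through MC events, playing animations with a movement lockout or ragdolling with a radial impulse.
; Modular body-part meshes follow the main mesh as master pose.
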(event `self.ReceiveTick`
  (params (DeltaSeconds :type "Float (single-precision)")))

(event `self.ReceiveBeginPlay`
  (`parent.ReceiveBeginPlay`)
  (set `self.Available` (not (`self.IsPlayerControlled`)))
  (bind _asbp_rbv_v_ai_pc (cast `/Game/Blueprints/Characters/BP_RBvV_AI_PC` (`AIBlueprintHelperLibrary.GetAIController` self))
    (:`then`
      (set `self.RBVV AI Controller` _asbp_rbv_v_ai_pc))
    (:`CastFailed`
      _))
  (bind _asw_player_hud (cast `/Game/Blueprints/UI/W_PlayerHUD` (`WidgetComponent.GetWidget` (`self.W_PlayerHUD`))))
  (set `self.Player HUD` _asw_player_hud))

(event `self.ReceivePossessed`
  (params (NewController :type "Controller Object Reference"))
  (bind _asbp_rbv_v_pc (cast `/Game/Blueprints/Characters/BP_RBvV_PC` NewController))
  (`/Game/Blueprints/UI/W_PlayerHUD.SetPlayerName` (`self.Player HUD`) (`KismetTextLibrary.Conv_IntToText` (`GameplayStatics.GetPlayerControllerID` _asbp_rbv_v_pc) false false))
  (set `self.Available` false)
  (set `self.RBVV Player Controller` _asbp_rbv_v_pc))

(event `self.ReceiveUnpossessed`
  (params (OldController :type "Controller Object Reference"))
  (set `self.Available` true)
  (`/Game/Blueprints/UI/W_PlayerHUD.SetPlayerName` (`self.Player HUD`) ""))

(event `SRV Punch`
  (params (AbilityClass :type "AblAbility Class Reference"))
  ;[1 1 1] Combat Attacks
  (`self.ActivateMeleeAttack` AbilityClass))

(event `PunchAttack`
  ;[1 1 1] Combat Attacks
  (`self.SRV Punch` (`self.PunchAbility`)))

(event `self.ReceiveAnyDamage`
  (params (Damage :type "Float (single-precision)") (DamageType :type "DamageType Object Reference") (InstigatedBy :type "Controller Object Reference") (DamageCauser :type "Actor Object Reference"))
  ;[1 1 1] On Damage taken
)

(event `SRV Kick`
  (params (AbilityClass :type "AblAbility Class Reference"))
  ;[1 1 1] Combat Attacks
  (`self.ActivateMeleeAttack` AbilityClass))

(event `KickAttack`
  ;[1 1 1] Combat Attacks
  (`self.SRV Kick` (`self.KickAbility`)))

(event `SRV Takedown`
  (params (AbilityClass :type "AblAbility Class Reference"))
  ;[1 1 1] Combat Attacks
  (`self.ActivateMeleeAttack` AbilityClass))

(event `TakedownAttack`
  ;[1 1 1] Combat Attacks
  (`self.SRV Takedown` (`KismetArrayLibrary.Array_Random` (`self.TakeDownAbilities`))))

(event `self.Set Is Dead`
  (params (Dead :type Boolean) (Killer :type "Actor Object Reference"))
  (`self.MC KillCharacter` Dead Killer))

(event `MC KillCharacter`
  (params (Dead :type Boolean) (Killer :type "Actor Object Reference"))
  (`self.KillCharacter` Dead Killer))

(event `self.HitReactions`
  (params (HitReaction :type "AnimSequence Object Reference") (InPosition :type "Float (single-precision)") (HitBy :type "Actor Object Reference"))
  (`self.MC HitReaction` HitReaction InPosition HitBy)
  (bind _isdead_ (`self.ReturnIsDead`))
  (if _isdead_
    (`self.Set Is Dead` true)
    (else
      (`KismetSystemLibrary.RetriggerableDelay` 5.0)
      (`self.AllowMovement` true))))

(event `MC HitReaction`
  (params (HitReaction :type "AnimSequence Object Reference") (InPosition :type "Float (double-precision)") (HitBy :type "Actor Object Reference"))
  (`self.IsHit` HitReaction InPosition HitBy))

(event `InputAxis|WalkForward`
  (params (AxisValue :type "Float (single-precision)"))
  (`self.MovementRestrictions`
    (:`Can Move`
      (`self.AddMovementInput` (1.0 0.0 0.0) AxisValue))))

(event `InputAxis|WalkRight`
  (params (AxisValue :type "Float (single-precision)"))
  (`self.MovementRestrictions`
    (:`Can Move`
      (`self.AddMovementInput` (0.0 1.0 0.0) AxisValue))))

(event `InputAction|Jump`
  (params (Key :type "Key Structure"))
  (:`Pressed`
    (`self.MovementRestrictions`
      (:`Can Move`
        (`self.Jump`)))))

(fn `ActivateMeleeAttack`
  (params (AbilityClass :type "AblAbility Class Reference"))
  (bind _returnvalue (`AblAbilityBlueprintLibrary.GetAbilityObjectFromClass` AbilityClass))
  (bind _abilitycomponent (`self.AbilityComponent`))
  (`/Engine/EditorBlueprintResources/StandardMacros.IsValid` _returnvalue
    (:`Is Valid`
      (set `self.CurrentAbility` _returnvalue)
      (bind _returnvalue_2 (`AblAbilityBlueprintLibrary.CreateAbilityContext` (`self.CurrentAbility`) _abilitycomponent))
      (`AblAbilityComponent.ActivateAbility` _abilitycomponent _returnvalue_2)
      (set `self.CurrentContext` _returnvalue_2)
      (`KismetSystemLibrary.PrintString` (`AblAbility.GetDisplayName` (`self.CurrentAbility`)) true true (struct :`A` 1.0) 5.0))))

(fn `AllowMovement`
  (params (`CanMove?` :type Boolean))
  (set `self.Allow Movement` `CanMove?`)
  (return))

(fn `CancelMeleeAttack`
  (params (AbilityClass :type "AblAbility Class Reference"))
  (bind _currentability (`self.CurrentAbility`))
  (`/Engine/EditorBlueprintResources/StandardMacros.IsValid` _currentability
    (:`Is Valid`
      (`AblAbilityContext.ClearTargetActors` (`self.CurrentContext`))
      (`AblAbilityComponent.CancelAbility` (`self.AbilityComponent`) _currentability "Successful"))))

(fn `IsHit`
  (params (HitReaction :type "AnimSequence Object Reference") (`Current Position` :type "Float (double-precision)") (HitBy :type "Actor Object Reference"))
  (bind _current_position (`local.Current Position`))
  (bind _mesh (`self.Mesh`))
  (if (`self.IsDead`)
    (`self.Set Is Dead` true (`local.HitBy`))
    (else
      (`MovementComponent.StopMovementImmediately` (`self.CharacterMovement`))
      (`self.AllowMovement` false)
      (`SkeletalMeshComponent.PlayAnimation` _mesh (`local.HitReaction`) false)
      (`SkeletalMeshComponent.SetPosition` _mesh (`KismetMathLibrary.RandomFloatInRange` (- _current_position 0.2) (+ _current_position 0.2)) true))))

(fn `IsUsingGamepad`
  (returns (UsingGamepad :type Boolean))
  (return false))

(fn `KillCharacter`
  (params (IsDead :type Boolean) (Killer :type "Actor Object Reference"))
  (bind _killer (`local.Killer`))
  (set `self.IsDead` IsDead)
  (message `/Game/Blueprints/Interfaces/BPI_AnimationInstance.IsDead?` (`SkeletalMeshComponent.GetAnimInstance` (`self.Mesh`)) false)
  (`MovementComponent.StopMovementImmediately` (`self.CharacterMovement`))
  (for _array_element (`self.K2_GetComponentsByClass` "/Script/Engine.SkeletalMeshComponent")
    (`PrimitiveComponent.SetCollisionProfileName` _array_element "DeadBody" true)
    (`PrimitiveComponent.SetSimulatePhysics` _array_element true))
  (`PrimitiveComponent.SetCollisionEnabled` (`self.GetComponentByClass` "/Script/Engine.CapsuleComponent") "NoCollision")
  (`/Engine/EditorBlueprintResources/StandardMacros.IsValid` _killer
    (:`Is Valid`
      (`PrimitiveComponent.AddRadialImpulse` (`self.Mesh`) (`self.K2_GetActorLocation` _killer) 250.0 20000.0 "RIF_Constant" false))
    (:`Is Not Valid`
      _))
  (cast `/Game/Blueprints/Characters/Vampires/BP_RBvV_AIPC_Vampire` (`self.RBVV AI Controller`))
  (`self.SetLifeSpan` 10.0))

(fn `MovementAllowed`
  (returns (`MovementAllowed?` :type Boolean))
  (return (`self.Allow Movement`)))

(fn `ReturnGender`
  (returns (ChracterGender :type "/Game/Blueprints/Enums/E_CharactersGenders Enum"))
  (return (`self.Chracter Gender`)))

(fn `ReturnIsDead`
  (returns (`IsDead?` :type Boolean))
  (return (`self.IsDead`)))

(fn `ReturnTeamID`
  (returns (TeamID :type Integer))
  (bind _teamid (message `/Game/Blueprints/Interfaces/BPI_CharacterAttributes.ReturnTeamID` (`self.GetController`)))
  (return (`KismetMathLibrary.Conv_ByteToInt` (`KismetMathLibrary.Conv_IntToByte` _teamid))))

(fn `UserConstructionScript`
  (`SkinnedMeshComponent.SetLeaderPoseComponent` (`self.SKM_Upper`) (`self.Mesh`) false)
  (`SkinnedMeshComponent.SetLeaderPoseComponent` (`self.SKM_Lower`) (`self.Mesh`) false)
  (`SkinnedMeshComponent.SetLeaderPoseComponent` (`self.SKM_Head`) (`self.Mesh`) false)
  (`SkinnedMeshComponent.SetLeaderPoseComponent` (`self.SKM_Hair`) (`self.Mesh`) false)
  (`SkinnedMeshComponent.SetLeaderPoseComponent` (`self.SKM_Hat`) (`self.Mesh`) false)
  (`SkinnedMeshComponent.SetLeaderPoseComponent` (`self.SKM_Eyewear`) (`self.Mesh`) false)
  (`SkinnedMeshComponent.SetLeaderPoseComponent` (`self.SKM_Gloves`) (`self.Mesh`) false)
  (`SkinnedMeshComponent.SetLeaderPoseComponent` (`self.SKM_Back`) (`self.Mesh`) false)
  (`SkinnedMeshComponent.SetLeaderPoseComponent` (`self.SKM_Weapon`) (`self.Mesh`) false)
  (`SkinnedMeshComponent.SetLeaderPoseComponent` (`self.SKM_Shoes`) (`self.Mesh`) false))