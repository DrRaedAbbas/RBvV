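; AI controller that assigns a team ID and drives its pawn through a configurable behavior tree, enabling movement avoidance on possession.
; Tick mirrors the pawn's death state to the blackboard and halts movement when it is dead or movement is disallowed.
; Perception updates replace a missing or dead target with the nearest perceived actor, if alive, writing it and its hostility to the blackboard.
; An older delayed chase-or-wander chain is left unconnected.
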(event `self.ReceiveBeginPlay`
  (`parent.ReceiveBeginPlay`)
  (`self.SRV SetTeamID` (`self.Custom Team ID`)))

(event `SRV SetTeamID`
  (params (NewTeamID :type Integer))
  (`self.SetGenericTeamId` (make `GenericTeamId` (`KismetMathLibrary.Conv_IntToByte` NewTeamID))))

(event `self.ReceivePossess`
  (params (PossessedPawn :type "Pawn Object Reference"))
  (`self.SRV SetTeamID` (`self.Custom Team ID`))
  (`CharacterMovementComponent.SetAvoidanceEnabled` (`self.GetComponentByClass` PossessedPawn "/Script/Engine.CharacterMovementComponent") true)
  (bind _btasset (`self.BTAsset`)
    (:`then`
      (`self.RunBehaviorTree` _btasset)
      (`self.UseBlackboard` (`self.Blackboard Asset`)))
    (:`else`)))

(event `self.ReceiveTick`
  (params (DeltaSeconds :type "Float (single-precision)"))
  (bind _returnvalue (`self.K2_GetPawn`))
  (`/Engine/EditorBlueprintResources/StandardMacros.IsValid` _returnvalue
    (:`Is Valid`
      (bind _isdead_ (message `/Game/Blueprints/Interfaces/BPI_CharacterAttributes.ReturnIsDead` _returnvalue))
      (bind _blackboard (`self.Blackboard`)
        (:`then`
          (`BlackboardComponent.SetValueAsBool` _blackboard "IsDead" _isdead_))
        (:`else`
          _))
      (if _isdead_
        (`Pawn.ConsumeMovementInputVector` _returnvalue :!label _label)
        (`self.StopMovement`)
        (else
          (bind _movementallowed_ (message `/Game/Blueprints/Interfaces/BPI_CharacterAttributes.MovementAllowed` (`self.K2_GetPawn`)))
          (if (not _movementallowed_)
            (goto _label)))))))

(event `self.AIPerception.OnPerceptionUpdated`
  (params (UpdatedActors :type "Array of Actor Object Reference (by ref)"))
  (bind (_distance _returnvalue) (`GameplayStatics.FindNearestActor` (`self.K2_GetActorLocation` (`self.K2_GetPawn`)) (`self.Updated Actors`)))
  (set `self.Updated Actors` UpdatedActors)
  (bind _targetactor (`self.TargetActor`)
    (:`then`
      (bind _isdead_ (message `/Game/Blueprints/Interfaces/BPI_CharacterAttributes.ReturnIsDead` _targetactor))
      (if _isdead_
        (`/Engine/EditorBlueprintResources/StandardMacros.IsValid` _returnvalue :!label _label_2
          (:`Is Valid`
            (bind _isdead__2 (message `/Game/Blueprints/Interfaces/BPI_CharacterAttributes.ReturnIsDead` _returnvalue))
            (if (not _isdead__2)
              (bind _info (`AIPerceptionComponent.GetActorsPerception` (`self.AIPerception`) _returnvalue))
              (bind (_target _lastsensedstimuli _bishostile) (break `ActorPerceptionBlueprintInfo` _info))
              (set `self.Is Hostile` _bishostile)
              (set `self.TargetActor` _target)
              (bind _blackboard (`self.Blackboard`)
                (:`then`
                  (`BlackboardComponent.SetValueAsBool` _blackboard "EnemyFound" (`self.Is Hostile`))
                  (`BlackboardComponent.SetValueAsObject` _blackboard "TargetActor" (`self.TargetActor`)))
                (:`else`)))))))
    (:`else`
      (goto _label_2))))

(fn `AllowMovement`
  (params (`CanMove?` :type Boolean))
  (message `/Game/Blueprints/Interfaces/BPI_CharacterAttributes.AllowMovement` (`self.K2_GetPawn`) `CanMove?`)
  (return))

(fn `IsUsingGamepad`
  (returns (UsingGamepad :type Boolean))
  (return false))

(fn `MovementAllowed`
  (returns (`MovementAllowed?` :type Boolean))
  (bind _movementallowed_ (message `/Game/Blueprints/Interfaces/BPI_CharacterAttributes.MovementAllowed` (`self.K2_GetPawn`)))
  (return _movementallowed_))

(fn `ReturnGender`
  (returns (ChracterGender :type "/Game/Blueprints/Enums/E_CharactersGenders Enum"))
  (return "NewEnumerator0"))

(fn `ReturnIsDead`
  (returns (`IsDead?` :type Boolean))
  (return false))

(fn `ReturnTeamID`
  (returns (TeamID :type Integer))
  (bind _returnvalue_teamid (break `GenericTeamId` (`self.GetGenericTeamId`)))
  (return (`KismetMathLibrary.Conv_ByteToInt` _returnvalue_teamid)))

(fn `UserConstructionScript`)