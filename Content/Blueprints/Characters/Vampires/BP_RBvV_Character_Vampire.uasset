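; Vampire character Blueprint that adds spawn and death effects and automatic despawning to its parent character.
; Spawn plays a random particle burst and reverses the dissolve timeline; death plays it forward with Niagara.
; The construction script shares dynamic materials across body parts and hair/hat for that dissolve.
; Each tick, when no player pawn is within DespawnDistance, it destroys itself if world-static geometry blocks a head-to-BP_Camera trace.
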(event `self.ReceiveBeginPlay`
  (`parent.ReceiveBeginPlay`)
  (`self.Spawn`))

(event `self.ReceiveTick`
  (params (DeltaSeconds :type "Float (single-precision)"))
  (`parent.ReceiveTick` DeltaSeconds)
  (if (not (`self.IsThereAnyClosePlayer`))
    (bind _returnvalue (`GameplayStatics.GetActorOfClass` "/Game/Blueprints/BP_Camera.BP_Camera_C"))
    (bind (_outhit _returnvalue_2) (`KismetSystemLibrary.LineTraceSingleForObjects` (`SceneComponent.K2_GetComponentLocation` (`self.SKM_Head`)) (`self.K2_GetActorLocation` _returnvalue) (`|MakeArray` "ObjectTypeQuery1" :!type "EObjectTypeQuery Enum")))
    (if _returnvalue_2
      (`self.K2_DestroyActor`))))

(event `/Game/Blueprints/Interfaces/BPI_CharacterAttributes.Set Is Dead`
  (params (Dead :type Boolean) (Killer :type "Actor Object Reference"))
  (`parent.Set Is Dead` Dead Killer)
  (`self.Dissolve`))

(event `Dissolve`
  ;[1 1 1] Dissolve FX
  (`ActorComponent.SetActive` (`self.Niagara`) true false)
  (bind (_direction _dissolvevalue) (`Timeline|DissolveFX-TM` :!via `PlayFromStart` :!label _label)
    (:`Update`
      (`MaterialInstanceDynamic.SetScalarParameterValue` (`self.Dissolve_BodyDynao_MAT`) "DissolveFX" _dissolvevalue)
      (`MaterialInstanceDynamic.SetScalarParameterValue` (`self.Dissolve_HairDynao_MAT`) "DissolveFX" _dissolvevalue))
    (:`Finished`
      (`ActorComponent.SetActive` (`self.Niagara`) false true))))

(event `Spawn`
  ;[1 1 1] Dissolve FX
  (`GameplayStatics.SpawnEmitterAtLocation` (`KismetArrayLibrary.Array_Random` (`|MakeArray` "/Game/ImpactFX/ParticleSystems/JangaFX/Par_Punch_Impact_01.Par_Punch_Impact_01" "/Game/ImpactFX/ParticleSystems/JangaFX/Par_Ground_Punch_Impact_03.Par_Ground_Punch_Impact_03" "/Game/ImpactFX/ParticleSystems/Fakado_Examples/Par_Aura_01.Par_Aura_01" "/Game/ImpactFX/ParticleSystems/Fakado_Examples/Par_Magic_Prison_01.Par_Magic_Prison_01" :!type "ParticleSystem Object Reference")) (+ (`SceneComponent.GetSocketLocation` (`self.Mesh`) "root") (0.0 0.0 5.0)))
  (goto _label :!via `ReverseFromEnd`))

(fn `IsThereAnyClosePlayer`
  (returns (`ClosePlayerFound?` :type Boolean))
  (locals (ClosePlayerFound :type Boolean))
  (bind _outactors (`GameplayStatics.GetAllActorsOfClass` "/Script/Engine.PlayerController"))
  (for _array_element _outactors
    (bind _returnvalue (`Controller.K2_GetPawn` _array_element))
    (`/Engine/EditorBlueprintResources/StandardMacros.IsValid` _returnvalue
      (:`Is Valid`
        (if (<= (`self.GetDistanceTo` _returnvalue self) (`self.DespawnDistance`))
          (set `local.ClosePlayerFound` true)
          (break)))))
  (return (`local.ClosePlayerFound`)))

(fn `UserConstructionScript`
  (bind _mesh (`self.Mesh`))
  (bind _skm_hair (`self.SKM_Hair`))
  (`parent.UserConstructionScript`)
  (bind _returnvalue (`PrimitiveComponent.CreateDynamicMaterialInstance` _mesh 0 null "None"))
  (bind _output_get (set `self.Dissolve_BodyDynao_MAT` _returnvalue))
  (`PrimitiveComponent.SetMaterial` _mesh 0 _output_get)
  (`PrimitiveComponent.SetMaterial` (`self.SKM_Head`) 0 _output_get)
  (`PrimitiveComponent.SetMaterial` (`self.SKM_Gloves`) 0 _output_get)
  (`PrimitiveComponent.SetMaterial` (`self.SKM_Head`) 1 _output_get)
  (bind _returnvalue_2 (`PrimitiveComponent.CreateDynamicMaterialInstance` _skm_hair 0 null "None"))
  (bind _output_get_2 (set `self.Dissolve_HairDynao_MAT` _returnvalue_2))
  (`PrimitiveComponent.SetMaterial` _skm_hair 0 _output_get_2)
  (`PrimitiveComponent.SetMaterial` (`self.SKM_Hat`) 0 _output_get_2))