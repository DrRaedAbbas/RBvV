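; Player controller for RBvV that lets a player take over and swap between available characters from the game mode's roster.
; StartToPlay possesses the first available character; four switch inputs pick by index, returning the previous character to its AI controller and updating ViewCamera's tracked characters.
; Punch, kick and takedown inputs forward to the current character.
; Team ID resets to 0 on possession, which also disables movement avoidance; offline possession logic is unreachable.
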(event `Key|NumPadZero`
  (params (Key :type "Key Structure"))
  (:`Pressed`
    (`self.SRV SetTeamID` 0)))

(event `Key|NumPadOne`
  (params (Key :type "Key Structure"))
  (:`Pressed`
    (`self.SRV SetTeamID` 1)))

(event `SRV SetTeamID`
  (params (NewTeamID :type Integer))
  (`self.SetGenericTeamId` (make `GenericTeamId` (`KismetMathLibrary.Conv_IntToByte` NewTeamID))))

(event `self.ReceiveBeginPlay`
  ;[1 1 1] BEGIN PLAY
  (`KismetSystemLibrary.Delay` 1.0)
  (bind _asbp_rbv_v_gm (cast `/Game/Blueprints/BP_RBvV_GM` (`GameplayStatics.GetGameMode`)))
  (bind _output_get (set `self.RBvV GM` _asbp_rbv_v_gm))
  (set `self.RBVVCharacters` (`/Game/Blueprints/BP_RBvV_GM.RBVVCharacters` _output_get))
  (`self.SRV SetTeamID` 0))

(event `PossessCharacter`
  ;[1 1 1] Possess Character
  (`/Engine/EditorBlueprintResources/StandardMacros.IsValid` (`self.K2_GetPawn`)
    (:`Is Not Valid`
      (bind _rbvv_gm (`self.RBvV GM`)
        (:`then`
          (for (_array_element _array_index) (`/Game/Blueprints/BP_RBvV_GM.RBVVCharacters` _rbvv_gm)
            (if (`/Game/Blueprints/Characters/BP_RBvV_Character.Available` _array_element)
              (bind _possesssuccess (`self.OnlinePossessNewCharacter` _array_index))
              (if _possesssuccess
                (break)))))
        (:`else`)))))

(event `UpdateCamera`
  (bind _returnvalue (`self.K2_GetPawn`))
  ;[1 1 1] Update the camera (calls after possess character)
  (`/Engine/EditorBlueprintResources/StandardMacros.IsValid` _returnvalue
    (:`Is Valid`
      (bind _output_get (set `self.CurrentRBVV Character` (cast `/Game/Blueprints/Characters/BP_RBvV_Character` _returnvalue :!pure true)))
      (`KismetArrayLibrary.Array_RemoveItem` (`/Game/Blueprints/BP_Camera.PlayerCharacters` (`self.ViewCamera`)) _output_get))
    (:`Is Not Valid`
      _))
  (bind _viewcamera (`self.ViewCamera`)
    (:`then`
      (`KismetArrayLibrary.Array_Add` (`/Game/Blueprints/BP_Camera.PlayerCharacters` _viewcamera) (`self.K2_GetPawn`))
      (`/Game/Blueprints/BP_Camera.UpdatePlayersAndCharacters` _viewcamera))
    (:`else`)))

(event `self.ReceivePossess`
  (params (PossessedPawn :type "Pawn Object Reference"))
  (`self.SRV SetTeamID` 0)
  (`CharacterMovementComponent.SetAvoidanceEnabled` (`self.GetComponentByClass` PossessedPawn "/Script/Engine.CharacterMovementComponent") false))

(event `Key|AnyKey` :consume false :paused true
  (params (Key :type "Key Structure"))
  (:`Pressed`
    (set `self.IsGamepad` (`KismetInputLibrary.Key_IsGamepadKey` Key))))

(event `InputAction|StartToPlay`
  (params (Key :type "Key Structure"))
  ;[1 1 1] Possess New Character / Swap Character
  (:`Pressed`
    (`self.PossessCharacter`)
    (`KismetSystemLibrary.Delay` 0.2)
    (`self.UpdateCamera` :!label _label)))

(event `InputAction|SwitchCharacter1`
  (params (Key :type "Key Structure"))
  ;[1 1 1] Possess New Character / Swap Character
  (:`Pressed`
    (`self.SRV SwapCharacter` 0)))

(event `InputAction|Punch`
  (params (Key :type "Key Structure"))
  ;[1 1 1] Combat
  (:`Pressed`
    (bind _currentrbvv_character (`self.CurrentRBVV Character`)
      (:`then`
        (`/Game/Blueprints/Characters/BP_RBvV_Character.PunchAttack` _currentrbvv_character))
      (:`else`))))

(event `InputAction|SwitchCharacter2`
  (params (Key :type "Key Structure"))
  ;[1 1 1] Possess New Character / Swap Character
  (:`Pressed`
    (`self.SRV SwapCharacter` 1)))

(event `SRV SwapCharacter`
  (params (CharacterIndex :type Integer))
  ;[1 1 1] Possess New Character / Swap Character
  (`self.OnlinePossessNewCharacter` CharacterIndex)
  (goto _label))

(event `InputAction|Kick`
  (params (Key :type "Key Structure"))
  ;[1 1 1] Combat
  (:`Pressed`
    (bind _currentrbvv_character (`self.CurrentRBVV Character`)
      (:`then`
        (`/Game/Blueprints/Characters/BP_RBvV_Character.KickAttack` _currentrbvv_character))
      (:`else`))))

(event `InputAction|SwitchCharacter3`
  (params (Key :type "Key Structure"))
  ;[1 1 1] Possess New Character / Swap Character
  (:`Pressed`
    (`self.SRV SwapCharacter` 2)))

(event `InputAction|Takedown`
  (params (Key :type "Key Structure"))
  ;[1 1 1] Combat
  (:`Pressed`
    (bind _currentrbvv_character (`self.CurrentRBVV Character`)
      (:`then`
        (`/Game/Blueprints/Characters/BP_RBvV_Character.TakedownAttack` _currentrbvv_character))
      (:`else`))))

(event `InputAction|SwitchCharacter4`
  (params (Key :type "Key Structure"))
  ;[1 1 1] Possess New Character / Swap Character
  (:`Pressed`
    (`self.SRV SwapCharacter` 3)))

(fn `GetAvailableCharacter`
  (params (CharacterID :type Integer))
  (returns (Chracter :type "/Game/Blueprints/Characters/BP_RBvV_Character Object Reference") (Available :type Boolean))
  (bind _rbvv_gm (`self.RBvV GM`)
    (:`then`
      (bind _output (`|GetArrayItem` (`/Game/Blueprints/BP_RBvV_GM.RBVVCharacters` _rbvv_gm) CharacterID))
      (return _output (`/Game/Blueprints/Characters/BP_RBvV_Character.Available` _output)))
    (:`else`)))

(fn `IsUsingGamepad`
  (returns (UsingGamepad :type Boolean))
  (return (`self.IsGamepad`)))

(fn `MovementAllowed`
  (returns (`MovementAllowed?` :type Boolean))
  (return false))

(fn `OfflinePossessNewCharacter`
  (params (CharacterIndex :type Integer))
  (returns (PossessSuccess :type Boolean))
  (locals (NewCharacter :type "/Game/Blueprints/Characters/BP_RBvV_Character Object Reference"))
  (bind _viewcamera (`self.ViewCamera`))
  (bind _output (`|GetArrayItem` (`self.RBVVCharacters`) CharacterIndex))
  (if (`/Game/Blueprints/Characters/BP_RBvV_Character.Available` _output)
    (bind _output_get (set `local.NewCharacter` _output))
    (`self.Possess` _output_get)
    (`self.SetViewTargetWithBlend` _viewcamera 1.0 "VTBlend_Linear" 1.0 true)
    (`KismetArrayLibrary.Array_Add` (`/Game/Blueprints/BP_Camera.PlayerCharacters` _viewcamera) (`local.NewCharacter`))
    (bind _currentrbvv_character (`self.CurrentRBVV Character`)
      (:`then`
        (`KismetArrayLibrary.Array_RemoveItem` (`/Game/Blueprints/BP_Camera.PlayerCharacters` (`self.ViewCamera`)) _currentrbvv_character))
      (:`else`
        _))
    (set `self.CurrentRBVV Character` (`local.NewCharacter`))
    (`/Engine/EditorBlueprintResources/StandardMacros.IsValid` (`self.K2_GetPawn`)
      (:`Is Valid`
        (return true))
      (:`Is Not Valid`
        (return false)))))

(fn `OnlinePossessNewCharacter`
  (params (CharacterIndex :type Integer))
  (returns (PossessSuccess :type Boolean))
  (locals (NewCharacter :type "/Game/Blueprints/Characters/BP_RBvV_Character Object Reference") (PreviousCharacter :type "/Game/Blueprints/Characters/BP_RBvV_Character Object Reference"))
  (bind (_chracter _available) (`self.GetAvailableCharacter` CharacterIndex))
  (if _available
    (set `local.NewCharacter` _chracter)
    (set `local.PreviousCharacter` (`self.CurrentRBVV Character`))
    (`self.Possess` (`local.NewCharacter`))
    (set `self.CurrentRBVV Character` (`local.NewCharacter`))
    (bind _previouscharacter (`local.PreviousCharacter`)
      (:`then`
        (`self.Possess` (`/Game/Blueprints/Characters/BP_RBvV_Character.RBVV AI Controller` _previouscharacter) _previouscharacter))
      (:`else`
        _))
    (`/Engine/EditorBlueprintResources/StandardMacros.IsValid` (`self.K2_GetPawn`)
      (:`Is Valid`
        (return true))
      (:`Is Not Valid`
        (return false)))))

(fn `ReturnGender`
  (returns (ChracterGender :type "/Game/Blueprints/Enums/E_CharactersGenders Enum"))
  (return "NewEnumerator0"))

(fn `ReturnIsDead`
  (returns (`IsDead?` :type Boolean))
  (return false))

(fn `ReturnTeamID`
  (returns (TeamID :type Integer))
  (bind _returnvalue_teamid (break `GenericTeamId` (`self.GetGenericTeamId`)))
  (return (`KismetMathLibrary.Conv_ByteToInt` _returnvalue_teamid)))

(fn `UserConstructionScript`)