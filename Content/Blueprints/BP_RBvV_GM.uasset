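; Game mode for RBvV that pits a four-member band (Anna, Dan, Pixie, Will) against vampires in local multiplayer.
; BeginPlay creates the HUD, spawns the band at player starts, adds three extra local controllers unless on a dedicated server, then possesses for player one.
; Tick tops vampires up to a cap at random navmesh points around the average position of player-controlled members, falling back to the whole band.
; CharacterDied clears that member's HUD slot.
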(event `self.ReceiveBeginPlay`
  (bind _returnvalue (`self.GetTransform` (`self.K2_FindPlayerStart` null)))
  (bind _returnvalue_2 (`|CreateWidget` "/Game/RBvV/HUD/InGameHUD.InGameHUD_C"))
  (bind _output_get (set `self.InGameHUD` _returnvalue_2))
  (`UserWidget.AddToViewport` _output_get 0)
  (`self.SpawnCharacter` "/Game/Blueprints/Characters/Band/Anna/BP_Anna.BP_Anna_C" _returnvalue "NewEnumerator1")
  (`self.SpawnCharacter` "/Game/Blueprints/Characters/Band/Dan/BP_Dan.BP_Dan_C" _returnvalue "NewEnumerator3")
  (`self.SpawnCharacter` "/Game/Blueprints/Characters/Band/Pixie/BP_Pixie.BP_Pixie_C" _returnvalue "NewEnumerator2")
  (`self.SpawnCharacter` "/Game/Blueprints/Characters/Band/Will/BP_Will.BP_Will_C" _returnvalue "NewEnumerator4")
  (`KismetSystemLibrary.Delay` 0.1)
  (`KismetArrayLibrary.Array_AddUnique` (`self.PlayerControllers`) (`GameplayStatics.GetPlayerController` 0))
  (if (not (`KismetSystemLibrary.IsDedicatedServer`))
    (for _ (range 1 4)
      (`self.SpawnNewPlayer`)))
  (`KismetSystemLibrary.Delay` 1.0)
  (`self.SetActorTickEnabled` true)
  (`self.PossesCharacter` 0))

(event `PossesCharacter`
  (params (ControllerIndex :type Integer))
  (bind _output (`|GetArrayItem` (`self.PlayerControllers`) ControllerIndex))
  (`/Game/Blueprints/Characters/BP_RBvV_PC.PossessCharacter` _output)
  (`/Game/Blueprints/Characters/BP_RBvV_PC.UpdateCurrentCharacter` _output))

(event `self.ReceiveTick`
  (params (DeltaSeconds :type "Float (single-precision)"))
  (bind _projectedlocation (`NavigationSystemV1.K2_ProjectPointToNavigation` (`NavigationSystemV1.K2_GetRandomLocationInNavigableRadius` (`self.GetAISpawnPoint`) 1000.0 null null)))
  (`KismetSystemLibrary.Delay` 0.0)
  (bind _outactors (`GameplayStatics.GetAllActorsOfClass` "/Game/Blueprints/Characters/Vampires/BP_RBvV_Character_Vampire.BP_RBvV_Character_Vampire_C"))
  (bind _output_get (set `self.VampiresCount` (- (`self.VampiresCountMax`) (`KismetArrayLibrary.Array_Length` _outactors))))
  (for _ (range 1 (+ _output_get 1))
    (`AIBlueprintHelperLibrary.SpawnAIFromClass` (`KismetArrayLibrary.Array_Random` (`self.Vampires`)) null (`KismetMathLibrary.MakeVector` (.x _projectedlocation) (.y _projectedlocation) (`KismetMathLibrary.FClamp` (.z _projectedlocation) 100.0 (.z _projectedlocation))) (`KismetMathLibrary.MakeRotator` 0.0 0.0 (`KismetMathLibrary.RandomFloatInRange` 0.0 360.0)) true null)))

(event `CharacterDied`
  (params (Item :type "/Game/Blueprints/Characters/BP_RBvV_Character Object Reference (by ref)"))
  (bind _ingamehud (`self.InGameHUD`))
  (bind _returnvalue (`KismetArrayLibrary.Array_RemoveItem` (`self.RBVVCharacters`) Item))
  (if _returnvalue
    (switch `/Game/Blueprints/Enums/E_BandName` (`/Game/Blueprints/Characters/BP_RBvV_Character.Name` Item)
      (:`NewEnumerator1`
        (set `/Game/RBvV/HUD/InGameHUD.Anna` null _ingamehud))
      (:`NewEnumerator2`
        (set `/Game/RBvV/HUD/InGameHUD.Pixie` null _ingamehud))
      (:`NewEnumerator3`
        (set `/Game/RBvV/HUD/InGameHUD.Dan` null _ingamehud))
      (:`NewEnumerator4`
        (set `/Game/RBvV/HUD/InGameHUD.Will` null _ingamehud)))))

(fn `GetAISpawnPoint`
  (returns (SpawnPoint :type "Vector Structure"))
  (locals (LocBandCharacters :type "Array of /Game/Blueprints/Characters/Band/BP_RBvV_Character_Band Object Reference"))
  (bind _locbandcharacters (`local.LocBandCharacters`))
  (bind _outactors (`GameplayStatics.GetAllActorsOfClass` "/Game/Blueprints/Characters/Band/BP_RBvV_Character_Band.BP_RBvV_Character_Band_C"))
  (for _array_element _outactors
    (if (`Pawn.IsPlayerControlled` _array_element)
      (`KismetArrayLibrary.Array_Add` (`local.LocBandCharacters`) _array_element)))
  (if (> (`KismetArrayLibrary.Array_Length` _locbandcharacters) 0)
    (bind _returnvalue (`GameplayStatics.GetActorArrayAverageLocation` _locbandcharacters))
    (return _returnvalue)
    (else
      (bind _returnvalue_2 (`GameplayStatics.GetActorArrayAverageLocation` _outactors))
      (return _returnvalue_2))))

(fn `SpawnCharacter`
  (params (CharacterClass :type "/Game/Blueprints/Characters/BP_RBvV_Character Class Reference") (SpawnTransform :type "Transform Structure") (Name :type "/Game/Blueprints/Enums/E_BandName Enum" :default "NewEnumerator0"))
  (returns (SpawnedCharacter :type "/Game/Blueprints/Characters/Band/BP_RBvV_Character_Band Object Reference"))
  (bind _ingamehud (`self.InGameHUD`))
  (bind _returnvalue (`|SpawnActorFromClass` CharacterClass SpawnTransform "AdjustIfPossibleButAlwaysSpawn" "OverrideRootScale" null null))
  (bind _asbp_rbv_v_character_band (cast `/Game/Blueprints/Characters/Band/BP_RBvV_Character_Band` _returnvalue))
  (`KismetArrayLibrary.Array_Add` (`self.RBVVCharacters`) _asbp_rbv_v_character_band)
  (bind _output_get (set `/Game/Blueprints/Characters/BP_RBvV_Character.Name` Name _asbp_rbv_v_character_band))
  (switch `/Game/Blueprints/Enums/E_BandName` _output_get
    (:`NewEnumerator1`
      (set `/Game/RBvV/HUD/InGameHUD.Anna` _asbp_rbv_v_character_band _ingamehud))
    (:`NewEnumerator2`
      (set `/Game/RBvV/HUD/InGameHUD.Pixie` _asbp_rbv_v_character_band _ingamehud))
    (:`NewEnumerator3`
      (set `/Game/RBvV/HUD/InGameHUD.Dan` _asbp_rbv_v_character_band _ingamehud))
    (:`NewEnumerator4`
      (set `/Game/RBvV/HUD/InGameHUD.Will` _asbp_rbv_v_character_band _ingamehud)))
  (return _asbp_rbv_v_character_band))

(fn `SpawnNewPlayer`
  (bind _returnvalue (`GameplayStatics.CreatePlayer` -1))
  (bind _asbp_rbv_v_pc (cast `/Game/Blueprints/Characters/BP_RBvV_PC` _returnvalue))
  (`KismetArrayLibrary.Array_AddUnique` (`self.PlayerControllers`) _asbp_rbv_v_pc)
  (set `/Game/Blueprints/Characters/BP_RBvV_PC.RBvV GM` self _asbp_rbv_v_pc)
  (bind _returnvalue_2 (`Controller.K2_GetPawn` _asbp_rbv_v_pc))
  (`/Engine/EditorBlueprintResources/StandardMacros.IsValid` _returnvalue_2
    (:`Is Valid`
      (`self.K2_DestroyActor` _returnvalue_2))))

(fn `UserConstructionScript`)